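; BP_Block is a Mario-style hit block that gives coins as a Brick or hearts as a Surprise Box, depending on BlockType.
; When the third-person character hits it, a timeline bumps the mesh upward, spawns the pickup at the Arrow and increments the character's Coins or Lives.
; Each bump decrements MaxCoins or MaxHearts, swapping to the EmptyBox mesh at zero.
; The construction script applies the configurable BlockModel mesh.
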(event `self.ReceiveBeginPlay`
  (bind _relativelocation (`SceneComponent.RelativeLocation` (`self.Model`)))
  ; Saving Locations
  (set `self.Original Location` _relativelocation)
  (set `self.NewLocation` (+ _relativelocation (0.0 0.0 10.0))))

(event `self.Model.OnComponentHit`
  (params (HitComponent :type "PrimitiveComponent Object Reference") (OtherActor :type "Actor Object Reference") (OtherComp :type "PrimitiveComponent Object Reference") (NormalImpulse :type "Vector Structure") (Hit :type "HitResult Structure (by ref)"))
  (bind _model (`self.Model`))
  (bind _returnvalue_location (`KismetMathLibrary.BreakTransform` (`SceneComponent.K2_GetComponentToWorld` (`self.Arrow`))))
  (bind _returnvalue_location_2 (`KismetMathLibrary.BreakTransform` (`SceneComponent.K2_GetComponentToWorld` (`self.Arrow`))))
  (bind _asbp_third_person_character (cast `/Game/ThirdPerson/Blueprints/BP_ThirdPersonCharacter` OtherActor))
  (switch `/Game/Blueprints/E_BlockType` (`self.BlockType`)
    (:`NewEnumerator0`
      (if (not (== (`self.MaxCoins`) 0))
        (bind (_direction _blockmovement) (`Timeline|Moveblock` :!via `PlayFromStart`)
          (:`Update`
            (`SceneComponent.K2_SetRelativeLocation` (`self.Model`) (`KismetMathLibrary.VLerp` (`self.Original Location`) (`self.NewLocation`) _blockmovement) false false))
          (:`Finished`
            (bind _result (`/Engine/EditorBlueprintResources/StandardMacros.DecrementInt` (`self.MaxCoins`))
              (:`  `
                (if (== _result 0)
                  (`StaticMeshComponent.SetStaticMesh` _model "/Game/Meshes/EmptyBox.EmptyBox" :!label _label)
                  (`SceneComponent.SetRelativeScale3D` _model (0.47 0.47 0.47))))))
          (:`SpawnTime`
            (`|SpawnActorFromClass` "/Game/Blueprints/BP_Coin.BP_Coin_C" (`KismetMathLibrary.MakeTransform` _returnvalue_location_2 (struct) (0.5 0.5 0.5)) "Undefined" "MultiplyWithRoot" null null)
            (`/Engine/EditorBlueprintResources/StandardMacros.IncrementInt` (`/Game/ThirdPerson/Blueprints/BP_ThirdPersonCharacter.Coins` _asbp_third_person_character))))))
    (:`NewEnumerator1`
      (if (not (== (`self.MaxHearts`) 0))
        (bind (_direction_2 _blockmovement_2) (`Timeline|Timeline` :!via `PlayFromStart`)
          (:`Update`
            (`SceneComponent.K2_SetRelativeLocation` (`self.Model`) (`KismetMathLibrary.VLerp` (`self.Original Location`) (`self.NewLocation`) _blockmovement_2) false false))
          (:`Finished`
            (bind _result_2 (`/Engine/EditorBlueprintResources/StandardMacros.DecrementInt` (`self.MaxHearts`))
              (:`  `
                (if (== _result_2 0)
                  (goto _label)))))
          (:`SpawnTime`
            (`|SpawnActorFromClass` "/Game/Blueprints/BP_Heart.BP_Heart_C" (`KismetMathLibrary.MakeTransform` _returnvalue_location (struct) (0.7 0.7 0.7)) "Undefined" "MultiplyWithRoot" null null)
            (`/Engine/EditorBlueprintResources/StandardMacros.IncrementInt` (`/Game/ThirdPerson/Blueprints/BP_ThirdPersonCharacter.Lives` _asbp_third_person_character))))))))

(fn `UserConstructionScript`
  (`StaticMeshComponent.SetStaticMesh` (`self.Model`) (`self.BlockModel`)))